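; BP_SkeletonGrunt is a skeleton melee enemy that detects, attacks and takes damage from the third-person player character.
; Pawn sensing sets the HasSeenPlayer blackboard key on its AI controller.
; Its attack event sphere-traces forward, playing the attack montage and applying damage only when the player is hit.
; A DoOnce ignores further damage during hit reactions; at zero health it plays a death montage, then destroys itself.
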(event `self.ReceiveAnyDamage`
  (params (Damage :type "Float (single-precision)") (DamageType :type "DamageType Object Reference") (InstigatedBy :type "Controller Object Reference") (DamageCauser :type "Actor Object Reference"))
  ;[1 1 1] DamageEvent
  (`/Engine/EditorBlueprintResources/StandardMacros.DoOnce` false :!label _label
    (:`Completed`
      (bind _output_get (set `self.Health` (- (`self.Health`) Damage)))
      (if (<= _output_get 0.0)
        (`self.PlayAnimMontage` "/Game/SkeletonCrew/Skeleton_Grunt/Animations/Skeleton_Grunt_Death_Montage.Skeleton_Grunt_Death_Montage")
        (`KismetSystemLibrary.PrintString` "Death" true true (struct :`R` 1.0 :`B` 0.110081 :`A` 1.0))
        (`KismetSystemLibrary.Delay` 2.0)
        (`self.K2_DestroyActor`)
        (else
          (bind _returnvalue (`self.PlayAnimMontage` "/Game/SkeletonCrew/Skeleton_Grunt/Animations/Skeleton_Grunt_Hit_Front_Montage.Skeleton_Grunt_Hit_Front_Montage"))
          (`KismetSystemLibrary.PrintString` "Damaged" true true (struct :`R` 1.0 :`B` 0.110081 :`A` 1.0))
          (`KismetSystemLibrary.Delay` _returnvalue)
          (goto _label :!via `Reset`))))))

(event `self.PawnSensing.OnSeePawn`
  (params (Pawn :type "Pawn Object Reference"))
  ;[1 1 1] OnSeeEvent
  (cast `/Game/ThirdPerson/Blueprints/BP_ThirdPersonCharacter` Pawn)
  (`BlackboardComponent.SetValueAsBool` (`AIBlueprintHelperLibrary.GetBlackboard` (`AIBlueprintHelperLibrary.GetAIController` self)) "HasSeenPlayer" true))

(event `AttackPlayerByGruntEvent`
  (bind _returnvalue (`self.K2_GetActorLocation`))
  ;[1 1 1] AttackPlayerEvent
  (bind (_outhit _returnvalue_2) (`KismetSystemLibrary.SphereTraceSingleForObjects` :`Start` _returnvalue :`End` (+ _returnvalue (* (`KismetMathLibrary.GetForwardVector` (`self.K2_GetActorRotation`)) 120.0)) :`Radius` 100.0 :`ObjectTypes` (`|MakeArray` "ObjectTypeQuery3" :!type "EObjectTypeQuery Enum") :`DrawDebugType` "ForDuration" :`DrawTime` 1.0))
  (if _returnvalue_2
    (bind (_bblockinghit _binitialoverlap _time _distance _location _impactpoint _normal _impactnormal _physmat _hitactor) (`GameplayStatics.BreakHitResult` _outhit))
    (cast `/Game/ThirdPerson/Blueprints/BP_ThirdPersonCharacter` _hitactor)
    (`self.PlayAnimMontage` "/Game/SkeletonCrew/Skeleton_Grunt/Animations/Skeleton_Grunt_Default_Attack_Montage.Skeleton_Grunt_Default_Attack_Montage")
    (`GameplayStatics.ApplyDamage` _hitactor 10.0)))

(fn `UserConstructionScript`)