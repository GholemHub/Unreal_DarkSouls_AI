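; Skeleton mage enemy that reports its state to an AI Blackboard and shows a health bar widget while the player is inside its sphere.
; Damage lowers health, updates the bar and flags LowHP, then either sets IsDead and disables capsule collision or plays a hit montage.
; A DoOnce ignores further damage until the montage length elapses.
; Pawn sensing pulses HasSeenPlayer for half a second when it sees the player.
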(event `self.ReceiveBeginPlay`
  (bind _aswbp_enemy_health_bar (cast `/Game/UI/WBP_EnemyHealthBar` (`WidgetComponent.GetUserWidgetObject` (`self.Widget`))))
  (set `self.As WBP Enemy Health Bar` _aswbp_enemy_health_bar))

(event `self.Sphere.OnComponentBeginOverlap`
  (params (OverlappedComponent :type "PrimitiveComponent Object Reference") (OtherActor :type "Actor Object Reference") (OtherComp :type "PrimitiveComponent Object Reference") (OtherBodyIndex :type Integer) (bFromSweep :type Boolean) (SweepResult :type "HitResult Structure (by ref)"))
  ;[1 1 1] Sphere health bar
  (cast `/Game/ThirdPerson/Blueprints/BP_ThirdPersonCharacter` OtherActor)
  (`SceneComponent.SetVisibility` (`self.Widget`) true false))

(event `self.Sphere.OnComponentEndOverlap`
  (params (OverlappedComponent :type "PrimitiveComponent Object Reference") (OtherActor :type "Actor Object Reference") (OtherComp :type "PrimitiveComponent Object Reference") (OtherBodyIndex :type Integer))
  ;[1 1 1] Sphere health bar
  (cast `/Game/ThirdPerson/Blueprints/BP_ThirdPersonCharacter` OtherActor)
  (`SceneComponent.SetVisibility` (`self.Widget`) false false))

(event `self.ReceiveAnyDamage`
  (params (Damage :type "Float (single-precision)") (DamageType :type "DamageType Object Reference") (InstigatedBy :type "Controller Object Reference") (DamageCauser :type "Actor Object Reference"))
  ;[1 1 1] DamageEvent
  (`/Engine/EditorBlueprintResources/StandardMacros.DoOnce` false :!label _label
    (:`Completed`
      (bind _output_get (set `self.Health` (- (`self.Health`) Damage)))
      (set `/Game/UI/WBP_EnemyHealthBar.Health` _output_get (`self.As WBP Enemy Health Bar`))
      (`self.SetLowHP`)
      (if (<= _output_get 0.0)
        (`self.SetIsDead` self)
        (`PrimitiveComponent.SetCollisionEnabled` (`self.CapsuleComponent`) "NoCollision")
        (else
          (bind _returnvalue (`self.PlayAnimMontage` "/Game/SkeletonCrew/Skeleton_Mage/Animations/Skeleton_Mage_Hit_Front_Montage.Skeleton_Mage_Hit_Front_Montage"))
          (`KismetSystemLibrary.Delay` _returnvalue)
          (goto _label :!via `Reset`))))))

(event `self.PawnSensing.OnSeePawn`
  (params (Pawn :type "Pawn Object Reference"))
  (bind _returnvalue (`AIBlueprintHelperLibrary.GetBlackboard` (`AIBlueprintHelperLibrary.GetAIController` self)))
  ;[1 1 1] OnSeeEvent
  (if (not (`BlackboardComponent.GetValueAsBool` _returnvalue "HasSeenPlayer"))
    (cast `/Game/ThirdPerson/Blueprints/BP_ThirdPersonCharacter` Pawn)
    (`BlackboardComponent.SetValueAsBool` _returnvalue "HasSeenPlayer" true)
    (`KismetSystemLibrary.Delay` 0.5)
    (`BlackboardComponent.SetValueAsBool` _returnvalue "HasSeenPlayer" false)))

(fn `SetIsDead`
  (params (Controller :type "Actor Object Reference"))
  (`BlackboardComponent.SetValueAsBool` (`AIBlueprintHelperLibrary.GetBlackboard` (`AIBlueprintHelperLibrary.GetAIController` Controller)) "IsDead" true))

(fn `SetLowHP`
  (`BlackboardComponent.SetValueAsBool` (`AIBlueprintHelperLibrary.GetBlackboard` (`AIBlueprintHelperLibrary.GetAIController` self)) "LowHP" (<= (`self.Health`) 20.0)))

(fn `UserConstructionScript`)